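; AIC_Enemy is the enemy AI controller, which targets the player's BP_Captain pawn.
; On BeginPlay it initializes BB_Enemy, runs BT_Enemy, then casts player pawn 0 to BP_Captain, leaving the target unset if the cast fails.
; SetAttackTarget writes the target to the blackboard and caches it in a variable.
; The target is assigned directly at startup, with no perception or Tick logic.
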(event EventBeginPlay
  (Class|AIController|UseBlackboard "/Game/Blueprints/AI/BB_Enemy.BB_Enemy")
  (AI|RunBehaviorTree "/Game/Blueprints/AI/BT_Enemy.BT_Enemy")
  (bind _asbp_captain (Utilities|Casting|CastToBP_Captain (Game|Player|GetPlayerPawn 0)))
  (CallFunction|SetAttackTarget _asbp_captain))

(event EventTick
  (params (DeltaSeconds :type Float%20%28single-precision%29)))

(fn ConstructionScript)

(fn SetAttackTarget
  (params (AttackTarget :type BP%20Captain%20Object%20Reference))
  (AI|Components|Blackboard|SetValueasObject (Variables|Default|GetBlackboard) (Variables|Default|GetAttackTargetKey) AttackTarget)
  (Variables|Default|SetAttackTarget AttackTarget))